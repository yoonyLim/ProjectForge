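; BP_AI is an NPC pawn that initializes its stats from data tables, then wanders randomly around the level.
; On BeginPlay, SetNPCVal looks up its InstanceName row and adds the "Blank" armor, weapon and shield rows into HP, JobVal and DefVal, also setting RoleName.
; After a short delay, RandomRoam repeatedly moves to nearby reachable points, pausing randomly after each success and retrying immediately on failure.
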(event `Random Roam`
  ;[1 1 1] Random Roam
  (`|AIMoveTo` self (`NavigationSystemV1.K2_GetRandomReachablePointInRadius` (`self.K2_GetActorLocation`) 1500.0 null null) null
    (:`OnSuccess`
      (`KismetSystemLibrary.Delay` (`KismetMathLibrary.RandomFloatInRange` 0.3 4.0))
      (`self.Random Roam`))
    (:`OnFail`
      (`self.Random Roam`))))

(event `self.ReceiveBeginPlay`
  (`self.Set NPC Val`)
  (`KismetSystemLibrary.Delay` 1.0)
  ;[1 1 1] Random Roam
  (`self.Random Roam`))

(event `Set NPC Val`
  ;[1 1 1] About Values
  (bind _returnvalue (`|GetDataTableRow` "/Game/Interaction/AI/DT_NPCValTable.DT_NPCValTable" (`self.Instance_Name`))
    (:`then`
      (bind _returnvalue_2 (`|GetDataTableRow` "/Game/Interaction/AI/DT_ArmorTable.DT_ArmorTable" "Blank")
        (:`then`
          (bind _returnvalue_3 (`|GetDataTableRow` "/Game/Interaction/AI/DT_WeaponTable.DT_WeaponTable" "Blank")
            (:`then`
              (bind _returnvalue_4 (`|GetDataTableRow` "/Game/Interaction/AI/DT_ShieldTable.DT_ShieldTable" "Blank")
                (:`then`
                  (bind (_hp _job_val _def_val _role_nm) (break `/Game/Interaction/AI/F_NPCData` _returnvalue))
                  (set `self.HP` (+ _hp (`.Equipment_val_3_B9568EF645054FC89A232F98F6C824CB` (break `/Game/Interaction/AI/F_ArmorData` _returnvalue_2))))
                  (set `self.Job_val` (+ _job_val (`.Weapon_val_4_503F990440D0CE74FBAF7F84E474E2DA` (break `/Game/Interaction/AI/F_WeaponData` _returnvalue_3))))
                  (set `self.Def_val` (+ _def_val (`.Shield_val_2_4590DCD7477368F10E6D38B968D192B7` (break `/Game/Interaction/AI/F_ShieldData` _returnvalue_4))))
                  (set `self.Role_Name` _role_nm))))))))))

(fn `UserConstructionScript`)