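; BP_NPCSpawnManager spawns a random selection of NPCs when play begins.
; It shuffles the row names of DT_NPCValTable and keeps up to the first 16, so each pick is a distinct row.
; For each name it spawns a BP_AI at the manager's own location, ignoring collision, passes the name as InstanceName and spawns its default controller.
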(event `self.ReceiveBeginPlay`
  (`self.Get Random NPC Names`)
  (for _array_element (`self.Selected_Names`)
    (bind _returnvalue (`|SpawnActorFromClass` "/Game/Interaction/AI/BP_AI.BP_AI_C" (`KismetMathLibrary.MakeTransform` (`self.K2_GetActorLocation`)) "AlwaysSpawn" "MultiplyWithRoot" null _array_element null))
    (`self.SpawnDefaultController` _returnvalue)))

(event `Get Random NPC Names`
  (bind _outrownames (`DataTableFunctionLibrary.GetDataTableRowNames` "/Game/Interaction/AI/DT_NPCValTable.DT_NPCValTable"))
  (bind _output_get (set `self.Out Row Names` _outrownames))
  (`KismetArrayLibrary.Array_Shuffle` _output_get)
  (for (_array_element _array_index) (`self.Out Row Names`)
    (if (<= _array_index 15)
      (`KismetArrayLibrary.Array_Add` (`self.Selected_Names`) _array_element)
      (else
        (break)))))

(fn `UserConstructionScript`)