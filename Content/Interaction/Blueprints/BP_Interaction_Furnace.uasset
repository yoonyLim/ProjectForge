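; Furnace interactable that switches the player between third-person play and a first-person furnace view with its own HUD.
; Interact stops movement, snaps the player to a facing arrow and creates the furnace widget with a back-reference; QuitInteraction reverses the view and prompts.
; Fade widgets and timed delays cover both transitions.
; A separate function writes the player's iron ore stack count to the HUD.
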(event `/Game/Interaction/I_Interact.Interact`
  (bind (_returnvalue_x _returnvalue_y _returnvalue_z) (`KismetMathLibrary.BreakVector` (`SceneComponent.K2_GetComponentLocation` (`self.FaceFurnaceArrow`))))
  (if (not (`self.IsInteracting`))
    ;[1 1 1] Transition to First Person
    (`Widget.RemoveFromParent` (`self.Interaction Prompt`))
    (bind _asbp_player (cast `/Game/Player/Blueprints/BP_Player` (`GameplayStatics.GetPlayerCharacter` 0)))
    (`MovementComponent.StopMovementImmediately` (`Character.CharacterMovement` _asbp_player))
    (`self.FadeIn`)
    (`KismetSystemLibrary.Delay` 0.25)
    (`SceneComponent.K2_SetWorldLocationAndRotation` (`Character.CapsuleComponent` _asbp_player) (`KismetMathLibrary.MakeVector` _returnvalue_x _returnvalue_y (+ _returnvalue_z 100.0)) (struct :`Yaw` 180.0) false false)
    (`/Game/Player/Blueprints/BP_Player.TransitionToFirstPersonPOV` _asbp_player)
    (`KismetSystemLibrary.Delay` 0.75)
    (bind _returnvalue (`|CreateWidget` "/Game/UI/Interaction/WB_QuitInteraction.WB_QuitInteraction_C"))
    (bind _output_get (set `self.Interaction Prompt` _returnvalue))
    (`UserWidget.AddToViewport` _output_get 0)
    (set `self.IsInteracting` true)
    (bind _returnvalue_2 (`|CreateWidget` "/Game/UI/Blacksmithing/WBP_Furnace.WBP_Furnace_C"))
    (bind _output_get_2 (set `self.FurnaceHUD` _returnvalue_2))
    (`/Game/UI/Blacksmithing/WBP_Furnace.UpdateHUD` _output_get_2)
    (`UserWidget.AddToViewport` _output_get_2 0)
    (set `/Game/UI/Blacksmithing/WBP_Furnace.OwningInteractionBP` self _output_get_2)))

(event `/Game/Interaction/I_Interact.QuitInteraction`
  (if (`self.IsInteracting`)
    (`Widget.RemoveFromParent` (`self.Interaction Prompt`))
    (`self.FadeIn`)
    (`Widget.RemoveFromParent` (`self.FurnaceHUD`))
    (`KismetSystemLibrary.Delay` 0.25)
    (bind _asbp_player (cast `/Game/Player/Blueprints/BP_Player` (`GameplayStatics.GetPlayerCharacter` 0)))
    (`/Game/Player/Blueprints/BP_Player.TransitionToThirdPersonPOV` _asbp_player)
    (`KismetSystemLibrary.Delay` 0.75)
    (bind _returnvalue (`|CreateWidget` "/Game/UI/Interaction/WB_Interact.WB_Interact_C"))
    (bind _output_get (set `self.Interaction Prompt` _returnvalue))
    (`UserWidget.AddToViewport` _output_get 0)
    (set `self.IsInteracting` false)))

(fn `FadeIn`
  (bind _returnvalue (`|CreateWidget` "/Game/UI/Interaction/WB_Fade.WB_Fade_C"))
  (`UserWidget.AddToViewport` _returnvalue 0)
  (`/Game/UI/Interaction/WB_Fade.Fade Anim` _returnvalue))

(fn `UpdateFurnaceHUD`
  (bind _asbp_player (cast `/Game/Player/Blueprints/BP_Player` (`GameplayStatics.GetPlayerCharacter` 0)))
  (bind _ores (`/Game/Player/Blueprints/BP_Player.GetOres` _asbp_player))
  (for _array_element _ores
    (bind (_name _description _thumbnail _itemclass _stacksize) (break `/Game/Inventory/F_ItemStruct` _array_element))
    (if (== _name (`KismetTextLibrary.Conv_StringToText` (`|GetEnumeratorNameAsString` (enumliteral `/Game/Inventory/E_OreNames` "NewEnumerator0"))))
      (set `TextBlock.Text` (`KismetTextLibrary.Conv_IntToText` _stacksize) (`/Game/UI/Blacksmithing/WBP_Furnace.NumIronOre` (`self.FurnaceHUD`))))))

(fn `UserConstructionScript`
  (`parent.UserConstructionScript`))