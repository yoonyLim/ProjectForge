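; BP_Interaction_Teleport is an interactable that teleports the player to a set TeleportLocation.
; On Interact, it casts the player character to BP_Player, adds a WB_Fade widget to the viewport and plays its fade animation.
; After a short delay that lets the fade run, it calls the player's Teleport to the location, raised along Z by a fixed offset.
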(event `self.Interact`
  (bind (_teleportlocation_x _teleportlocation_y _teleportlocation_z) (`KismetMathLibrary.BreakVector` (`self.TeleportLocation`)))
  (bind _asbp_player (cast `/Game/Player/Blueprints/BP_Player` (`GameplayStatics.GetPlayerCharacter` 0)))
  (bind _returnvalue (`|CreateWidget` "/Game/UI/Interaction/WB_Fade.WB_Fade_C"))
  (`UserWidget.AddToViewport` _returnvalue 0)
  (`/Game/UI/Interaction/WB_Fade.Fade Anim` _returnvalue)
  (`KismetSystemLibrary.Delay` 0.3)
  (`self.K2_TeleportTo` :`self` _asbp_player :`DestLocation` (`KismetMathLibrary.MakeVector` _teleportlocation_x _teleportlocation_y (+ _teleportlocation_z 200.0))))

(fn `UserConstructionScript`
  (`parent.UserConstructionScript`))