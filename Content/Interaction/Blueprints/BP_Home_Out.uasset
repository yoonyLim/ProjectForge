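; BP_Home_Out is an interactable that moves the player to a fixed location, apparently as the exit from the home.
; A trigger box shows an interaction prompt widget, created at BeginPlay, while the player character overlaps it.
; The Interact event spawns a fade widget, plays its animation, waits briefly, then teleports the third-person character to hard-coded coordinates.
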(event `self.ReceiveBeginPlay`
  (bind _returnvalue (`|CreateWidget` "/Game/Interaction/WB_Interact.WB_Interact_C"))
  (set `self.Interaction Prompt` _returnvalue))

(event `self.Trigger Box.OnComponentBeginOverlap`
  (params (OverlappedComponent :type "PrimitiveComponent Object Reference") (OtherActor :type "Actor Object Reference") (OtherComp :type "PrimitiveComponent Object Reference") (OtherBodyIndex :type Integer) (bFromSweep :type Boolean) (SweepResult :type "HitResult Structure (by ref)"))
  (if (== OtherActor (`GameplayStatics.GetPlayerCharacter` 0))
    (`UserWidget.AddToViewport` (`self.Interaction Prompt`) 0)))

(event `self.Trigger Box.OnComponentEndOverlap`
  (params (OverlappedComponent :type "PrimitiveComponent Object Reference") (OtherActor :type "Actor Object Reference") (OtherComp :type "PrimitiveComponent Object Reference") (OtherBodyIndex :type Integer))
  (if (== (`GameplayStatics.GetPlayerCharacter` 0) OtherActor)
    (`Widget.RemoveFromParent` (`self.Interaction Prompt`))))

(event `self.Interact`
  (bind _asbp_third_person_character (cast `/Game/ThirdPerson/Blueprints/BP_ThirdPersonCharacter` (`GameplayStatics.GetPlayerCharacter` 0)))
  (bind _returnvalue (`|CreateWidget` "/Game/Interaction/WB_Fade.WB_Fade_C"))
  (`UserWidget.AddToViewport` _returnvalue 0)
  (`/Game/Interaction/WB_Fade.Fade Anim` _returnvalue)
  (`KismetSystemLibrary.Delay` 0.3)
  (`self.K2_TeleportTo` :`self` _asbp_third_person_character :`DestLocation` (370.0 370.0 150.0)))

(fn `UserConstructionScript`)