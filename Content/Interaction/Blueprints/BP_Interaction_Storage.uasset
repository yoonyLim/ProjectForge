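; Interactable storage Blueprint that shows the player's inventory and its own storage inventory when interacted with.
; On BeginPlay it creates its own WB_PlayerHUD widget, adds it to the viewport and keeps the reference.
; Interact uses that HUD to display the player inventory, then passes BPCInventorySystem to it to display the storage contents.
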(event `self.ReceiveBeginPlay`
  (`parent.ReceiveBeginPlay`)
  (bind _returnvalue (`|CreateWidget` "/Game/UI/WB_PlayerHUD.WB_PlayerHUD_C"))
  (bind _output_get (set `self.HUD` _returnvalue))
  (`UserWidget.AddToViewport` _output_get 0))

(event `self.Interact`
  (bind _hud (`self.HUD`))
  (`/Game/UI/WB_PlayerHUD.DisplayPlayerInventory` _hud)
  (`/Game/UI/WB_PlayerHUD.DisplayStorageInventory` _hud (`self.BPC_InventorySystem`)))

(fn `UserConstructionScript`
  (`parent.UserConstructionScript`))